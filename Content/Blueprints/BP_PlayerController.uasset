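; BP_PlayerController is a player controller for what appears to be a budgeted room-assignment game played with cursor or touch.
; The construction script enables the mouse cursor along with click, touch and mouse-over events, and BeginPlay copies InitBudget into Budget.
; IsRoomValid maps a room-use enum to the Bedroom, Livingroom, Kitchen or Bathroom reference and checks that it exists.
; SetRoom takes a use and a cube but has an empty body.
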(event EventBeginPlay
  (Variables|Default|SetBudget (Variables|Default|GetInitBudget)))

(fn ConstructionScript
  (bind _self self)
  (Variables|/Script/Engine.PlayerController|SetbShowMouseCursor _self true)
  (Variables|/Script/Engine.PlayerController|SetbEnableMouseOverEvents _self true)
  (Variables|/Script/Engine.PlayerController|SetbEnableClickEvents _self true)
  (Variables|Default|SetbEnableTouchEvents true))

(fn IsRoomValid
  (params (Use :type ECurrentUse%20Enum :default "NewEnumerator4"))
  (return (Math|Boolean|ORBoolean (and (Utilities|Enum|Equal(Enum) Use "NewEnumerator2") (Utilities|IsValid (Variables|Default|Getbedroom))) (and (Utilities|Enum|Equal(Enum) Use "NewEnumerator0") (Utilities|IsValid (Variables|Default|Getlivingroom))) (and (Utilities|Enum|Equal(Enum) Use "NewEnumerator1") (Utilities|IsValid (Variables|Default|Getkitchen))) (and (Utilities|Enum|Equal(Enum) Use "NewEnumerator3") (Utilities|IsValid (Variables|Default|Getbathroom))))))

(fn SetRoom
  (params (Use :type ECurrentUse%20Enum :default "NewEnumerator4") (Cube :type BP%20Cube%20Space%20Object%20Reference)))