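; BP_GameMode sets up the starting gardens on the level's grid of BP_CubeSpace actors.
; On BeginPlay it sets its own CurrentUse, gathers every cube space, switches randomly picked ones to another use, then updates every cube.
; Random picks can repeat, so the garden count may fall short of GardenNumInit.
; The construction script also updates whatever cubes are already in its Cubes array.
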(event EventBeginPlay
  (Variables|Default|SetCurrentUse "NewEnumerator4")
  (CallFunction|CreateInitGardens))

(fn ConstructionScript
  (CallFunction|UpdateGameCubes))

(fn CreateInitGardens
  (bind _outactors (Actor|GetAllActorsOfClass "/Game/Blueprints/BP_CubeSpace.BP_CubeSpace_C"))
  (bind _output_get (Variables|Default|SetCubes _outactors))
  (Utilities|FlowControl|Sequence
    (:then_0
      (for _index (range 0 (- (Variables|Default|GetGardenNumInit) 1))
        (Variables|/Game/Blueprints/BP_CubeSpace.BP_CubeSpace_C|SetCurrentUse (Utilities|Array|Get(acopy) (Variables|Default|GetCubes) (Math|Random|RandomIntegerinRange 0 (- (Utilities|Array|Length _output_get) 1))) "NewEnumerator5")))
    (:then_1
      (for _array_element _output_get
        (Default|UpdateCube _array_element)))))

(fn UpdateGameCubes
  (for _array_element (Variables|Default|GetCubes)
    (Default|UpdateCube _array_element)))