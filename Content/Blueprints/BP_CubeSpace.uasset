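; Clickable grid cell in a budget-based house layout game, where the player assigns the GameMode's selected room use.
; Sphere overlaps find four neighbours at BeginPlay; hovering the floor shows a wireframe cube.
; Clicks start or extend attached room actors, log the action, spend budget and call GameMode's UpdateGameCubes.
; UpdateCube tints walls by use or spawns gardens, hiding walls between same-use cells and using door meshes between different occupied uses.
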(event OnBeginCursorOver(floor)
  (params (TouchedComponent :type Primitive%20Component%20Object%20Reference))
  (Rendering|SetVisibility (Variables|Default|GetintCube) true false))

(event OnEndCursorOver(floor)
  (params (TouchedComponent :type Primitive%20Component%20Object%20Reference))
  (Rendering|SetVisibility (Variables|Default|GetintCube) false false))

(event OnClicked(floor)
  (params (TouchedComponent :type Primitive%20Component%20Object%20Reference) (ButtonPressed :type Key%20Structure))
  (if (> (Variables|/Game/Blueprints/BP_PlayerController.BP_PlayerController_C|GetBudget (Variables|Default|GetPlayerController)) 0.0)
    (CallFunction|EvaluatePlayerDecision)
    (bind _asbp_game_mode (Utilities|Casting|CastToBP_GameMode (Game|GetGameMode)))
    (Default|UpdateGameCubes _asbp_game_mode)))

(event EventBeginPlay
  (Rendering|SetVisibility (Variables|Default|GetintCube) false false)
  (CallFunction|SetComponentVisibility true false false false false)
  (bind _returnvalue (Rendering|Material|CreateDynamicMaterialInstance (Variables|Default|GetintCube) 0 "/Game/Materials/M_Wireframe.M_Wireframe" "None" :!class /Script/Engine.PrimitiveComponent))
  (Variables|Default|SetcubeMaterial _returnvalue)
  (bind _asbp_game_mode (Utilities|Casting|CastToBP_GameMode (Game|GetGameMode)))
  (Variables|Default|SetGameMode _asbp_game_mode)
  (CallFunction|SetNeighbours)
  (CallFunction|SetStaringCollisions)
  (bind _asbp_player_controller (Utilities|Casting|CastToBP_PlayerController (Game|GetPlayerController 0)))
  (Variables|Default|SetPlayerController _asbp_player_controller))

(event EventDestroyed
  (bind _children (CallFunction|GetAllAttachedActors self))
  (for _array_element _children
    (Actor|DestroyActor _array_element)))

(fn ConstructionScript
  (bind _walls (Variables|Default|Getwalls))
  (Utilities|Array|Add _walls (Variables|Default|Getwall1))
  (Utilities|Array|Add _walls (Variables|Default|Getwall2))
  (Utilities|Array|Add _walls (Variables|Default|Getwall3))
  (Utilities|Array|Add _walls (Variables|Default|Getwall4))
  (CallFunction|UpdateCube)
  (Variables|Default|SetisCubeExpandable true))

(fn SetComponentVisibility
  (params (floor :type Boolean) (wall1 :type Boolean) (wall2 :type Boolean) (wall3 :type Boolean) (wall4 :type Boolean))
  (Utilities|FlowControl|Sequence
    (:then_0
      (Rendering|SetVisibility (Variables|Default|Getfloor) floor false))
    (:then_1
      (Rendering|SetVisibility (Variables|Default|Getwall1) wall1 false))
    (:then_2
      (Rendering|SetVisibility (Variables|Default|Getwall2) wall2 false))
    (:then_3
      (Rendering|SetVisibility (Variables|Default|Getwall3) wall3 false))
    (:then_4
      (Rendering|SetVisibility (Variables|Default|Getwall4) wall4 false))))

(fn UpdateUse
  (if (not (Utilities|Enum|Equal(Enum) (Variables|Default|GetCurrentUse) "NewEnumerator4"))
    (Rendering|SetVisibility (Variables|Default|GetintCube) false false)
    (Utilities|FlowControl|Sequence
      (:then_0
        (for _array_element (Variables|Default|Getwalls)
          (bind _returnvalue (Rendering|Material|CreateDynamicMaterialInstance _array_element 0 0 "None" :!class /Script/Engine.PrimitiveComponent))
          (if (Utilities|Enum|Equal(Enum) (Variables|Default|GetCurrentUse) "NewEnumerator0")
            (Rendering|Material|SetVectorParameterValue _returnvalue "color" "(R=0.156189,G=0.937500,B=0.700392,A=1.000000)" :!class /Script/Engine.MaterialInstanceDynamic)
            (elif (Utilities|Enum|Equal(Enum) (Variables|Default|GetCurrentUse) "NewEnumerator1")
              (Rendering|Material|SetVectorParameterValue _returnvalue "color" "(R=0.589222,G=0.184976,B=0.937500,A=1.000000)" :!class /Script/Engine.MaterialInstanceDynamic)
              (elif (Utilities|Enum|Equal(Enum) (Variables|Default|GetCurrentUse) "NewEnumerator2")
                (Rendering|Material|SetVectorParameterValue _returnvalue "color" "(R=0.170417,G=0.937500,B=0.189135,A=1.000000)" :!class /Script/Engine.MaterialInstanceDynamic)
                (elif (Utilities|Enum|Equal(Enum) (Variables|Default|GetCurrentUse) "NewEnumerator3")
                  (Rendering|Material|SetVectorParameterValue _returnvalue "color" "(R=0.937500,G=0.104612,B=0.169964,A=1.000000)" :!class /Script/Engine.MaterialInstanceDynamic)
                  (elif (Utilities|Enum|Equal(Enum) (Variables|Default|GetCurrentUse) "NewEnumerator5")
                    (if (not (Variables|Default|GetisGarden))
                      (CallFunction|SetComponentVisibility false false false false false)
                      (bind _returnvalue_2 (Game|SpawnActorfromClass "/Game/Blueprints/Rooms/BP_Garden.BP_Garden_C" (Math|Transform|MakeTransform (Transformation|GetActorLocation) "0, 0, 0" "1,1,1") "Undefined" 0 0))
                      (Transformation|AttachActorToActor _returnvalue_2 self "None" "KeepWorld" "KeepWorld" "KeepWorld" true)
                      (Variables|Default|SetisGarden true))))))))))))

(fn SetNeighbours
  (Utilities|FlowControl|Sequence
    (:then_0
      (bind _asbp_cube_space (Utilities|Casting|CastToBP_CubeSpace (Utilities|Array|Get(acopy) (Collision|GetOverlappingActors (Variables|Default|GetSphere) "BP_CubeSpace_C" :!class /Script/Engine.PrimitiveComponent))))
      (bind _output_get (Variables|Default|SetNeighbour01 _asbp_cube_space))
      (Utilities|Array|Add (Variables|Default|GetNeighbours) _output_get))
    (:then_1
      (bind _asbp_cube_space_2 (Utilities|Casting|CastToBP_CubeSpace (Utilities|Array|Get(acopy) (Collision|GetOverlappingActors (Variables|Default|GetSphere1) "BP_CubeSpace_C" :!class /Script/Engine.PrimitiveComponent))))
      (bind _output_get_2 (Variables|Default|SetNeighbour02 _asbp_cube_space_2))
      (Utilities|Array|Add (Variables|Default|GetNeighbours) _output_get_2))
    (:then_2
      (bind _asbp_cube_space_3 (Utilities|Casting|CastToBP_CubeSpace (Utilities|Array|Get(acopy) (Collision|GetOverlappingActors (Variables|Default|GetSphere2) "BP_CubeSpace_C" :!class /Script/Engine.PrimitiveComponent))))
      (bind _output_get_3 (Variables|Default|SetNeighbour03 _asbp_cube_space_3))
      (Utilities|Array|Add (Variables|Default|GetNeighbours) _output_get_3))
    (:then_3
      (bind _asbp_cube_space_4 (Utilities|Casting|CastToBP_CubeSpace (Utilities|Array|Get(acopy) (Collision|GetOverlappingActors (Variables|Default|GetSphere3) "BP_CubeSpace_C" :!class /Script/Engine.PrimitiveComponent))))
      (bind _output_get_4 (Variables|Default|SetNeighbour04 _asbp_cube_space_4))
      (Utilities|Array|Add (Variables|Default|GetNeighbours) _output_get_4))))

(fn UpdateneighbourRelations
  (if (not (Utilities|Enum|Equal(Enum) (Variables|Default|GetCurrentUse) "NewEnumerator5"))
    (Utilities|FlowControl|Sequence
      (:then_0
        (Rendering|SetVisibility (Variables|Default|Getfloor) true false))
      (:then_1
        (CallFunction|UpdateWalls (Variables|Default|GetNeighbour01) (Variables|Default|Getwall1) (Variables|Default|Getwall01Root) "/Game/Geometry/wallDoor01.wallDoor01"))
      (:then_2
        (CallFunction|UpdateWalls (Variables|Default|GetNeighbour02) (Variables|Default|Getwall2) (Variables|Default|Getwall02Root) "/Game/Geometry/wallDoor02.wallDoor02"))
      (:then_3
        (CallFunction|UpdateWalls (Variables|Default|GetNeighbour03) (Variables|Default|Getwall3) (Variables|Default|Getwall03Root) "/Game/Geometry/wallDoor03.wallDoor03"))
      (:then_4
        (CallFunction|UpdateWalls (Variables|Default|GetNeighbour04) (Variables|Default|Getwall4) (Variables|Default|Getwall04Root) "/Game/Geometry/wallDoor04.wallDoor04")))))

(fn UpdateCube
  (Utilities|FlowControl|Sequence
    (:then_0
      (CallFunction|UpdateUse))
    (:then_1
      (if (Utilities|Enum|NotEqual(Enum) (Variables|Default|GetCurrentUse) "NewEnumerator4")
        (CallFunction|UpdateneighbourRelations)))))

(fn SetStaringCollisions
  (Utilities|FlowControl|Sequence
    (:then_0
      (Collision|SetCollisionEnabled (Variables|Default|GetintCube) "NoCollision"))
    (:then_2
      (Collision|SetCollisionEnabled (Variables|Default|Getwall1) "NoCollision"))
    (:then_3
      (Collision|SetCollisionEnabled (Variables|Default|Getwall2) "NoCollision"))
    (:then_4
      (Collision|SetCollisionEnabled (Variables|Default|Getwall3) "NoCollision"))
    (:then_5
      (Collision|SetCollisionEnabled (Variables|Default|Getwall4) "NoCollision"))))

(fn InstantiateRooms
  (bind _self self)
  (bind _self_2 self)
  (bind _self_3 self)
  (bind _self_4 self)
  (if (Utilities|Enum|Equal(Enum) (Variables|/Game/Blueprints/BP_GameMode.BP_GameMode_C|GetCurrentUse (Variables|Default|GetGameMode)) "NewEnumerator2")
    (bind _returnvalue (Game|SpawnActorfromClass "/Game/Blueprints/Rooms/BP_Bedroom.BP_Bedroom_C" (Math|Transform|MakeTransform (Transformation|GetActorLocation) "0, 0, 0" "1,1,1") "Undefined" 0 0))
    (Variables|/Game/Blueprints/BP_PlayerController.BP_PlayerController_C|Setbedroom (Variables|Default|GetPlayerController) _returnvalue)
    (Transformation|AttachActorToActor _returnvalue _self_2 "None" "KeepWorld" "KeepWorld" "KeepWorld" true)
    (Utilities|Array|Add (Variables|/Game/Blueprints/Rooms/BP_Bedroom.BP_Bedroom_C|GetMyCubes _returnvalue) _self_2)
    (Development|PrintString "NewBedroom")
    (elif (Utilities|Enum|Equal(Enum) (Variables|/Game/Blueprints/BP_GameMode.BP_GameMode_C|GetCurrentUse (Variables|Default|GetGameMode)) "NewEnumerator0")
      (bind _returnvalue_2 (Game|SpawnActorfromClass "/Game/Blueprints/Rooms/BP_LivingRoom.BP_LivingRoom_C" (Math|Transform|MakeTransform (Transformation|GetActorLocation) "0, 0, 0" "1,1,1") "Undefined" 0 0))
      (Variables|/Game/Blueprints/BP_PlayerController.BP_PlayerController_C|Setlivingroom (Variables|Default|GetPlayerController) _returnvalue_2)
      (Transformation|AttachActorToActor _returnvalue_2 _self_3 "None" "KeepRelative" "KeepRelative" "KeepRelative" true)
      (Utilities|Array|Add (Variables|/Game/Blueprints/Rooms/BP_LivingRoom.BP_LivingRoom_C|GetMyCubes _returnvalue_2) _self_3)
      (Development|PrintString "NewLiving")
      (elif (Utilities|Enum|Equal(Enum) (Variables|/Game/Blueprints/BP_GameMode.BP_GameMode_C|GetCurrentUse (Variables|Default|GetGameMode)) "NewEnumerator1")
        (bind _returnvalue_3 (Game|SpawnActorfromClass "/Game/Blueprints/Rooms/BP_Kitchen.BP_Kitchen_C" (Math|Transform|MakeTransform (Transformation|GetActorLocation) "0, 0, 0" "1,1,1") "Undefined" 0 0))
        (Variables|/Game/Blueprints/BP_PlayerController.BP_PlayerController_C|Setkitchen (Variables|Default|GetPlayerController) _returnvalue_3)
        (Transformation|AttachActorToActor _returnvalue_3 _self_4 "None" "KeepRelative" "KeepRelative" "KeepRelative" true)
        (Utilities|Array|Add (Variables|/Game/Blueprints/Rooms/BP_Kitchen.BP_Kitchen_C|GetMyCubes _returnvalue_3) _self_4)
        (Development|PrintString "NewKitchen")
        (elif (Utilities|Enum|Equal(Enum) (Variables|/Game/Blueprints/BP_GameMode.BP_GameMode_C|GetCurrentUse (Variables|Default|GetGameMode)) "NewEnumerator3")
          (bind _returnvalue_4 (Game|SpawnActorfromClass "/Game/Blueprints/Rooms/BP_Bathroom.BP_Bathroom_C" (Math|Transform|MakeTransform (Transformation|GetActorLocation) "0, 0, 0" "1,1,1") "Undefined" 0 0))
          (Variables|/Game/Blueprints/BP_PlayerController.BP_PlayerController_C|Setbathroom (Variables|Default|GetPlayerController) _returnvalue_4)
          (Transformation|AttachActorToActor _returnvalue_4 _self "None" "KeepRelative" "KeepRelative" "KeepRelative" true)
          (Utilities|Array|Add (Variables|/Game/Blueprints/Rooms/BP_Bathroom.BP_Bathroom_C|GetMyCubes _returnvalue_4) _self)
          (Development|PrintString "NewBathroom"))))))

(fn EvaluatePlayerDecision
  (bind _playercontroller (Variables|Default|GetPlayerController))
  (if (Utilities|Enum|NotEqual(Enum) (Variables|/Game/Blueprints/BP_GameMode.BP_GameMode_C|GetCurrentUse (Variables|Default|GetGameMode)) "NewEnumerator4")
    (Utilities|Array|Clear (LocalVariables|GetSameUseNeighbours))
    (for _array_element (Variables|Default|GetNeighbours)
      (if (Utilities|Enum|Equal(Enum) (Variables|/Game/Blueprints/BP_GameMode.BP_GameMode_C|GetCurrentUse (Variables|Default|GetGameMode)) (Variables|BP_CubeSpace_C|GetCurrentUse _array_element))
        (Utilities|Array|Add (LocalVariables|GetSameUseNeighbours) 0)))
    (if (and (== (Utilities|Array|Length (LocalVariables|GetSameUseNeighbours)) 0) (not (Default|IsRoomValid (Variables|Default|GetPlayerController) (Variables|/Game/Blueprints/BP_GameMode.BP_GameMode_C|GetCurrentUse (Variables|Default|GetGameMode)))))
      (CallFunction|InstantiateRooms)
      (CallFunction|SetCurrentUseandPayerAction)
      (Variables|/Game/Blueprints/BP_PlayerController.BP_PlayerController_C|SetBudget _playercontroller (- (Variables|/Game/Blueprints/BP_PlayerController.BP_PlayerController_C|GetBudget _playercontroller) 1e+02) :!label _label)
      (elif (!= (Utilities|Array|Length (LocalVariables|GetSameUseNeighbours)) 0)
        (CallFunction|ExpandRooms)
        (CallFunction|SetCurrentUseandPayerAction)
        (goto _label)))))

(fn SetCurrentUseandPayerAction
  (bind _gamemode (Variables|Default|GetGameMode))
  (bind _playeractions (Variables|/Game/Blueprints/BP_GameMode.BP_GameMode_C|GetPlayerActions _gamemode))
  (if (not (Utilities|Enum|Equal(Enum) (Variables|/Game/Blueprints/BP_GameMode.BP_GameMode_C|GetCurrentUse _gamemode) "NewEnumerator4"))
    (Variables|Default|SetCurrentUse (Variables|/Game/Blueprints/BP_GameMode.BP_GameMode_C|GetCurrentUse _gamemode))
    (Variables|Default|SetID (Utilities|Array|Length _playeractions))
    (Utilities|Array|Add _playeractions (Transformation|GetActorLocation))
    (Utilities|Array|Add (Variables|/Game/Blueprints/BP_GameMode.BP_GameMode_C|GetPlayerActionUse _gamemode) (Variables|Default|GetCurrentUse))
    (Rendering|Material|SetMaterial (Variables|Default|Getfloor) 0 "/Game/Materials/M_Wood_Floor_Walnut_Polished_2.M_Wood_Floor_Walnut_Polished_2")))

(fn ExpandRooms
  (bind _playercontroller (Variables|Default|GetPlayerController))
  (bind _playercontroller_2 (Variables|Default|GetPlayerController))
  (bind _playercontroller_3 (Variables|Default|GetPlayerController))
  (bind _playercontroller_4 (Variables|Default|GetPlayerController))
  (bind _bedroom (Variables|/Game/Blueprints/BP_PlayerController.BP_PlayerController_C|Getbedroom _playercontroller))
  (bind _livingroom (Variables|/Game/Blueprints/BP_PlayerController.BP_PlayerController_C|Getlivingroom _playercontroller_2))
  (bind _kitchen (Variables|/Game/Blueprints/BP_PlayerController.BP_PlayerController_C|Getkitchen _playercontroller_4))
  (bind _bathroom (Variables|/Game/Blueprints/BP_PlayerController.BP_PlayerController_C|Getbathroom _playercontroller_3))
  (if (Utilities|Enum|Equal(Enum) (Variables|/Game/Blueprints/BP_GameMode.BP_GameMode_C|GetCurrentUse (Variables|Default|GetGameMode)) "NewEnumerator2")
    (if (Utilities|IsValid _bedroom)
      (Utilities|Array|Add (Variables|/Game/Blueprints/Rooms/BP_Bedroom.BP_Bedroom_C|GetMyCubes _bedroom) self))
    (elif (Utilities|Enum|Equal(Enum) (Variables|/Game/Blueprints/BP_GameMode.BP_GameMode_C|GetCurrentUse (Variables|Default|GetGameMode)) "NewEnumerator0")
      (if (Utilities|IsValid _livingroom)
        (Utilities|Array|Add (Variables|/Game/Blueprints/Rooms/BP_LivingRoom.BP_LivingRoom_C|GetMyCubes _livingroom) self))
      (elif (Utilities|Enum|Equal(Enum) (Variables|/Game/Blueprints/BP_GameMode.BP_GameMode_C|GetCurrentUse (Variables|Default|GetGameMode)) "NewEnumerator1")
        (if (Utilities|IsValid _kitchen)
          (Utilities|Array|Add (Variables|/Game/Blueprints/Rooms/BP_Kitchen.BP_Kitchen_C|GetMyCubes _kitchen) self))
        (elif (Utilities|Enum|Equal(Enum) (Variables|/Game/Blueprints/BP_GameMode.BP_GameMode_C|GetCurrentUse (Variables|Default|GetGameMode)) "NewEnumerator3")
          (if (Utilities|IsValid _bathroom)
            (Utilities|Array|Add (Variables|/Game/Blueprints/Rooms/BP_Bathroom.BP_Bathroom_C|GetMyCubes _bathroom) self)))))))

(fn UpdateWalls
  (params (Neighbour :type BP%20Cube%20Space%20Object%20Reference) (Wall :type Static%20Mesh%20Component%20Object%20Reference) (wallRoot :type Scene%20Component%20Object%20Reference) (wallDoor :type Static%20Mesh%20Object%20Reference))
  (bind _currentuse (Variables|BP_CubeSpace_C|GetCurrentUse Neighbour))
  (Utilities|IsValid Neighbour
    (:Is%20Valid
      (if (Utilities|Enum|Equal(Enum) _currentuse (Variables|Default|GetCurrentUse))
        (Rendering|SetVisibility Wall false false)
        (else
          (Rendering|SetVisibility Wall true false)
          (if (not (Utilities|Enum|Equal(Enum) _currentuse "NewEnumerator4"))
            (Components|StaticMesh|SetStaticMesh Wall wallDoor)
            (if (< (Variables|BP_CubeSpace_C|GetID Neighbour) (Variables|Default|GetID))
              (Transformation|SetRelativeRotation wallRoot "0,180.000000, 0" false false))))))
    (:Is%20Not%20Valid
      (Rendering|SetVisibility Wall true false))))